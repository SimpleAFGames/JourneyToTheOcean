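; Player character for a 2D side-scrolling shooter, handling Enhanced Input movement, jumping and shooting.
; Pressing shoot fires a regular projectile; releasing fires a partial or full charge shot by hold time, unless damaged meanwhile.
; Shots spend ShotEnergy using per-class costs.
; Enemy capsule overlaps deal damage, triggering knockback, a stun animation that blocks move and shoot, and flickering invincibility that ignores Pawn collision.
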(event `self.ReceiveBeginPlay`
  (`parent.ReceiveBeginPlay`)
  (`|ExecutionSequence`
    (:`then_0`
      (bind _asplayer_controller (cast `PlayerController` (`self.GetController`)))
      (`EnhancedInputSubsystemInterface.AddMappingContext` (pcsubsystem `EnhancedInputLocalPlayerSubsystem` _asplayer_controller) "/Game/inputs/IMC_Action.IMC_Action" 0 (struct)))
    (:`then_1`
      (set `self.BaseLateralFriction` (`CharacterMovementComponent.FallingLateralFriction` (`self.CharacterMovement`))))))

(event `EnhancedInput|/Game/inputs/Action/IA_Jump`
  (params (ActionValue :type Boolean) (ElapsedSeconds :type "Float (double-precision)") (TriggeredSeconds :type "Float (double-precision)") (InputAction :type "InputAction Object Reference" :default "/Game/inputs/Action/IA_Jump.IA_Jump"))
  (:`Started`
    (`self.Jump`))
  (:`Canceled`
    (`self.StopJumping` :!label _label))
  (:`Completed`
    (goto _label)))

(event `EnhancedInput|/Game/inputs/Action/IA_Move`
  (params (ActionValue :type "Float (double-precision)") (ElapsedSeconds :type "Float (double-precision)") (TriggeredSeconds :type "Float (double-precision)") (InputAction :type "InputAction Object Reference" :default "/Game/inputs/Action/IA_Move.IA_Move"))
  (:`Triggered`
    (if (not (`self.Stun`))
      (`self.AddMovementInput` (1.0 0.0 0.0) ActionValue)
      (`self.Update rotation` ActionValue))))

(event `EnhancedInput|/Game/inputs/Action/IA_Shoot`
  (params (ActionValue :type Boolean) (ElapsedSeconds :type "Float (double-precision)") (TriggeredSeconds :type "Float (double-precision)") (InputAction :type "InputAction Object Reference" :default "/Game/inputs/Action/IA_Shoot.IA_Shoot"))
  (:`Started`
    (if (not (`self.Stun`))
      (set `self.WashitDuringCharge` false)
      (`self.SpawnProjectile` "/Game/BluePrints/Projectiles/Player/BP_PlayerProjectile_REGULAR.BP_PlayerProjectile_REGULAR_C")))
  (:`Completed`
    (if (not (`self.Stun`))
      (`self.Try Chargeshot` ElapsedSeconds))))

(event `self.CapsuleComponent.OnComponentBeginOverlap`
  (params (OverlappedComponent :type "PrimitiveComponent Object Reference") (OtherActor :type "Actor Object Reference") (OtherComp :type "PrimitiveComponent Object Reference") (OtherBodyIndex :type Integer) (bFromSweep :type Boolean) (SweepResult :type "HitResult Structure (by ref)"))
  (bind _asbpenimy_base (cast `/Game/BluePrints/Character/Enimy/BPEnimy_BASE` OtherActor))
  (if (== (`Character.CapsuleComponent` _asbpenimy_base) OtherComp)
    (`GameplayStatics.ApplyDamage` self (`self.OverlapDMG`) null _asbpenimy_base)))

(event `TriggerInvinibility`
  (`PrimitiveComponent.SetCollisionResponseToChannel` (`self.CapsuleComponent`) "ECC_Pawn" "ECR_Ignore")
  (bind _returnvalue (`KismetSystemLibrary.K2_SetTimerDelegate` (`|CreateDelegate` :!event `ToggleSpriteFlicker`) (`self.SpriteFlickerintervol`) true))
  (set `self.Flicker` _returnvalue)
  (`KismetSystemLibrary.RetriggerableDelay` (`self.InvicibilityDeley`))
  (`KismetSystemLibrary.K2_ClearAndInvalidateTimerHandle` (`self.Flicker`))
  (`PrimitiveComponent.SetCollisionResponseToChannel` (`self.CapsuleComponent`) "ECC_Pawn" "ECR_Overlap")
  (`SceneComponent.SetVisibility` (`self.Sprite`) true true))

(event `self.ReceiveAnyDamage`
  (params (Damage :type "Float (single-precision)") (DamageType :type "DamageType Object Reference") (InstigatedBy :type "Controller Object Reference") (DamageCauser :type "Actor Object Reference"))
  (bind _returnvalue_x (`KismetMathLibrary.BreakVector` (`KismetMathLibrary.GetForwardVector` (`KismetMathLibrary.FindLookAtRotation` (`self.K2_GetActorLocation`) (`self.K2_GetActorLocation` DamageCauser)))))
  (`parent.ReceiveAnyDamage` Damage DamageType InstigatedBy DamageCauser)
  (set `self.WashitDuringCharge` true)
  (`self.TriggerInvinibility`)
  (set `CharacterMovementComponent.FallingLateralFriction` 0.0 (`self.CharacterMovement`))
  (`self.LaunchCharacter` (`KismetMathLibrary.MakeVector` (* (`KismetMathLibrary.SelectFloat` -1.0 1.0 (> _returnvalue_x 0.0)) (`self.KnockBackPower`)) 0.0 (`self.KnockBackVert`)) true true)
  (`PaperZDAnimInstance.JumpToNode` (`PaperZDAnimationComponent.AnimInstance` (`self.AnimationComponent`)) "JumpStun" "None")
  (set `self.Stun` true)
  (`|ExecutionSequence`
    (:`then_0`
      (`KismetSystemLibrary.RetriggerableDelay` (`self.InvicibilityDeley`))
      (set `CharacterMovementComponent.FallingLateralFriction` (`self.BaseLateralFriction`) (`self.CharacterMovement`)))
    (:`then_1`
      (`KismetSystemLibrary.RetriggerableDelay` (`self.StunDurration`))
      (set `self.Stun` false))))

(event `TriggerShootAnim`
  (set `self.Isshooting` true)
  (`KismetSystemLibrary.RetriggerableDelay` (`self.ShootanimDurration`))
  (set `self.Isshooting` false))

(fn `restoreShotEnergy`
  (params (ProjectileClass :type "/Game/BluePrints/Projectiles/Player/BP_PlayerProjectile_BASE Class Reference (by ref)"))
  (set `self.ShotEnergy` (`KismetMathLibrary.Min` (+ (`self.ShotEnergy`) (`BlueprintMapLibrary.Map_Find` (`self.projectile2Energy`) (`local.ProjectileClass`))) (`self.MaxShotEnergy`))))

(fn `SpawnProjectile`
  (params (ProjectileClass :type "/Game/BluePrints/Projectiles/Player/BP_PlayerProjectile_BASE Class Reference"))
  (bind _shootpulse (`self.ShootPulse`))
  (if (>= (`self.ShotEnergy`) (`BlueprintMapLibrary.Map_Find` (`self.projectile2Energy`) (`local.ProjectileClass`)))
    (set `self.ShotEnergy` (`KismetMathLibrary.Max` (- (`self.ShotEnergy`) (`BlueprintMapLibrary.Map_Find` (`self.projectile2Energy`) (`local.ProjectileClass`)))))
    (`|SpawnActorFromClass` (`local.ProjectileClass`) (`KismetMathLibrary.MakeTransform` (`SceneComponent.K2_GetComponentLocation` _shootpulse) (`SceneComponent.K2_GetComponentRotation` _shootpulse)) "AlwaysSpawn" "MultiplyWithRoot" self self)
    (`self.TriggerShootAnim`)))

(fn `ToggleSpriteFlicker`
  (`SceneComponent.SetVisibility` (`self.Sprite`) (not (`SceneComponent.bVisible` (`self.Sprite`))) true))

(fn `Try Chargeshot`
  (params (eleapsedTime :type "Float (double-precision)"))
  (if (not (`self.WashitDuringCharge`))
    (if (>= (`local.eleapsedTime`) (`self.PartialChargeTime`))
      (if (>= (`local.eleapsedTime`) (`self.FullChargeTime`))
        (`self.SpawnProjectile` "/Game/BluePrints/Projectiles/Player/BP_Projectile_FullCharge.BP_Projectile_FullCharge_C")
        (else
          (`self.SpawnProjectile` "/Game/BluePrints/Projectiles/Player/BP_PlayerProjectile_partialCharge.BP_PlayerProjectile_partialCharge_C"))))))

(fn `Update rotation`
  (params (Direction :type "Float (double-precision)"))
  (`Controller.SetControlRotation` (`self.GetController`) (select `bool` (>= Direction 0.0) :`false` (`KismetMathLibrary.MakeRotator` 0.0 0.0 180.0) :`true` (`KismetMathLibrary.MakeRotator` 0.0))))

(fn `UserConstructionScript`
  (`parent.UserConstructionScript`))