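; BPC_Vitality is a health component that tracks an actor's current health and defeat state.
; On BeginPlay it sets CurrentHealth to MaxHealth.
; ReciveDamage subtracts damage, clamps the result between zero and MaxHealth, and sets IsDefeated once health reaches zero.
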(event `self.ReceiveBeginPlay`
  (set `self.CurrentHealth` (`self.MaxHealth`)))

(fn `ReciveDamage`
  (params (Damage :type "Float (double-precision)"))
  (set `self.CurrentHealth` (`KismetMathLibrary.FClamp` (- (`self.CurrentHealth`) Damage) 0.0 (`self.MaxHealth`)))
  (if (<= (`self.CurrentHealth`) 0.0)
    (set `self.IsDefeated` true)))